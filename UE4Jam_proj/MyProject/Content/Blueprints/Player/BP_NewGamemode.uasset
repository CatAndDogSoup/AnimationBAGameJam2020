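; Game mode that respawns the first-person player character and sets up the crosshair HUD.
; On BeginPlay it binds to the character's OnDestroyed event, hides the mouse cursor and adds a Crosshair widget to the viewport.
; When the character is destroyed, it waits briefly, spawns a replacement at the SpawnTransform variable and possesses it.
; It then calls Respawn to rebind the destroyed event, keeping the loop going.
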(event `Respawn`
  (bind _asbp_first_person_character (cast `/Game/Blueprints/Player/BP_FirstPersonCharacter` (`GameplayStatics.GetPlayerCharacter` 0) :!label _label))
  (add `self.OnDestroyed` _asbp_first_person_character (delegate `PlayerDestroyed`)))

(event `self.ReceiveBeginPlay`
  (bind _returnvalue (`GameplayStatics.GetPlayerController` 0))
  (`|ExecutionSequence`
    (:`then_0`
      (goto _label))
    (:`then_1`
      (set `PlayerController.bShowMouseCursor` false _returnvalue)
      (bind _returnvalue_2 (`|CreateWidget` "/Game/Blueprints/UserInterface/Crosshair.Crosshair_C" _returnvalue))
      (`UserWidget.AddToViewport` _returnvalue_2 0))))

(event `PlayerDestroyed` :!signature `self.OnDestroyed`
  (params (DestroyedActor :type "Actor Object Reference"))
  (`KismetSystemLibrary.Delay` 0.2)
  (bind _returnvalue (`|SpawnActorFromClass` "/Game/Blueprints/Player/BP_FirstPersonCharacter.BP_FirstPersonCharacter_C" (`self.SpawnTransform`) "Undefined" "OverrideRootScale" null null))
  (`Controller.Possess` (`GameplayStatics.GetPlayerController` 0) _returnvalue)
  (`self.Respawn`))

(fn `UserConstructionScript`)