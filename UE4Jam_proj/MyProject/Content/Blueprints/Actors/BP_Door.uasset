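; BP_Door is a double sliding door that opens once its LockCount equals LockCountRequired.
; Tick polls that condition, and a DoOnce caches target positions by offsetting each panel along its forward vector, in opposite directions, by DoorMoveAmount.
; After a short delay, a timeline lerps each panel from its current location toward its target, so the blend compounds each update.
; No closing logic or LockCount changes appear here.
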(event `self.ReceiveTick`
  (params (DeltaSeconds :type "Float (single-precision)"))
  (bind _left_door (`self.Left_door`))
  (bind _right_door (`self.Right_door`))
  (bind _returnvalue (`SceneComponent.K2_GetComponentLocation` _right_door))
  (bind _returnvalue_2 (`SceneComponent.K2_GetComponentLocation` _left_door))
  (if (== (`self.LockCount`) (`self.LockCountRequired`))
    (`|ExecutionSequence`
      (:`then_0`
        (`/Engine/EditorBlueprintResources/StandardMacros.DoOnce` false
          (:`Completed`
            (bind _output_get (set `self.RightDoorOpenValue` (+ _returnvalue (* (`SceneComponent.GetForwardVector` _right_door) (* (`self.DoorMoveAmount`) -1.0)))))
            (bind _output_get_2 (set `self.LeftDoorOpenValue` (+ _returnvalue_2 (* (`SceneComponent.GetForwardVector` _left_door) (`self.DoorMoveAmount`))))))))
      (:`then_1`
        (`KismetSystemLibrary.Delay` 0.3)
        (bind (_direction _lerp) (`Timeline|Timeline_0`)
          (:`Update`
            (`|ExecutionSequence`
              (:`then_0`
                (`SceneComponent.K2_SetWorldLocation` (`self.Right_door`) (`KismetMathLibrary.VLerp` _returnvalue _output_get _lerp) false false))
              (:`then_1`
                (`SceneComponent.K2_SetWorldLocation` (`self.Left_door`) (`KismetMathLibrary.VLerp` _returnvalue_2 _output_get_2 _lerp) false false)))))))))

(fn `UserConstructionScript`)