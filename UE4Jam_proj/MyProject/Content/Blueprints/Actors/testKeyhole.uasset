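; Keyhole actor that accepts one specific Key actor on overlap and counts toward unlocking a linked BP_Door.
; It swaps the destroyed key for its own KeyForLock mesh at the same pose, then a timeline lerps that mesh into its original slot.
; When the timeline finishes, it sets Locked to true and increments the door's LockCount.
; The construction script gives KeyForLock and KeyGuide the key's mesh and material.
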(event `self.ReceiveActorBeginOverlap`
  (params (OtherActor :type "Actor Object Reference"))
  (bind _key (`self.Key`))
  (bind _keyforlock (`self.KeyForLock`))
  ;[1 1 1] Get Key location and replace with the key for the lock. Update lock state to unlocked.
  (if (== OtherActor _key)
    (set `self.KeySlot` (`SceneComponent.K2_GetComponentToWorld` (`self.KeyForLock`)))
    (`SceneComponent.K2_SetWorldLocationAndRotation` _keyforlock (`self.K2_GetActorLocation` _key) (`self.K2_GetActorRotation` _key) false false)
    (`SceneComponent.SetVisibility` _keyforlock true false)
    (`self.K2_DestroyActor` (`self.Key`))
    (bind (_direction _lerp0_1) (`Timeline|LerpAlpha` :!via `PlayFromStart`)
      (:`Update`
        (`SceneComponent.K2_SetWorldTransform` (`self.KeyForLock`) (`KismetMathLibrary.TLerp` (`SceneComponent.K2_GetComponentToWorld` (`self.KeyForLock`)) (`self.KeySlot`) _lerp0_1) false false))
      (:`Finished`
        (set `self.Locked` true)
        ;[1 1 1] Cast +1 to BP door (needs to be less hardcoded)
        (bind _asbp_door (cast `/Game/Blueprints/Actors/BP_Door` (`self.WhatUnlocks`)))
        (set `/Game/Blueprints/Actors/BP_Door.LockCount` (+ (`/Game/Blueprints/Actors/BP_Door.LockCount` _asbp_door) 1) _asbp_door)))))

(fn `UserConstructionScript`
  (bind _keyforlock (`self.KeyForLock`))
  (bind _keyguide (`self.KeyGuide`))
  ;[1 1 1] Make the lockkey look like the key
  (`StaticMeshComponent.SetStaticMesh` _keyforlock (`self.KeyMesh`))
  (`PrimitiveComponent.SetMaterial` _keyforlock 0 (`self.KeyMaterial`))
  ;[1 1 1] Make the key guide look like the key
  (`StaticMeshComponent.SetStaticMesh` _keyguide (`self.KeyMesh`))
  (`PrimitiveComponent.SetMaterial` _keyguide 0 (`self.KeyMaterial`)))